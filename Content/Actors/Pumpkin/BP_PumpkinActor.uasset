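; Pumpkin actor Blueprint that handles UI and audio feedback for a pumpkin's growing, harvestable and evil states.
; State events clear and show the matching widgets: water bar with timer, harvest pop-up or evil health bar.
; Tick refreshes water or health percentage for the current state.
; Evil state start and end both pass IsEvil to the PC_Pumpkin controller and play the same evil sound.
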(event `self.ReceiveBeginPlay`
  (`self.Clear Widgets`))

(event `self.ReceiveTick`
  (params (DeltaSeconds :type "Float (single-precision)"))
  (switch `PumpkinState` (`self.CurrentPumpkinState`)
    (:`Growing`
      (`self.Update Water Level`))
    (:`Evil`
      (`self.Update Damage Level`))))

(event `self.OnPumpkinHarvested`
  (`SceneComponent.SetVisibility` (`self.Harvestable pop up`) false false))

(event `self.OnPumpkinHarvestStateStarted`
  (`self.Clear Widgets`)
  (`SceneComponent.SetVisibility` (`self.Harvestable pop up`) true false))

(event `self.OnPumpkinEvilStateStarted`
  (`self.Clear Widgets`)
  (`SceneComponent.SetVisibility` (`self.Evil_Health_Bar`) true false)
  (`self.SetIsEvil` :!label _label)
  (`GameplayStatics.PlaySound2D` "/Game/Sounds/5_-_Power-EVIL_ish_.5_-_Power-EVIL_ish_" 0.34 0.85 0.0 null null))

(event `self.OnPumpkinEvilStateEnd`
  (goto _label))

(event `self.OnPumpkinGrowingStateStarted`
  (`self.Clear Widgets`)
  (`SceneComponent.SetVisibility` (`self.Water_Level_Bar_Widget`) true false)
  (`SceneComponent.SetVisibility` (`self.Growing Timer`) true false))

(fn `Clear Widgets`
  (`SceneComponent.SetVisibility` (`self.Evil_Health_Bar`) false false)
  (`SceneComponent.SetVisibility` (`self.Harvestable pop up`) false false)
  (`SceneComponent.SetVisibility` (`self.Water_Level_Bar_Widget`) false false)
  (`SceneComponent.SetVisibility` (`self.Growing Timer`) false false))

(fn `SetIsEvil`
  (bind _aspc_pumpkin (cast `/Game/Actors/Pumpkin/PC_Pumpkin` (`self.GetController`)))
  (`/Game/Actors/Pumpkin/PC_Pumpkin.SetIsEvil` _aspc_pumpkin (`self.bIsEvil`)))

(fn `Update Damage Level`
  (bind _asevil_pumpkin_hp_bar (cast `/Game/UI/UI_Widgets/Evil_Pumpkin_HP_Bar` (`WidgetComponent.GetWidget` (`self.Evil_Health_Bar`))))
  (`ProgressBar.SetPercent` (`/Game/UI/UI_Widgets/Evil_Pumpkin_HP_Bar.Evil_Pumkin_Health` _asevil_pumpkin_hp_bar) (/ (`self.CurrentHealth`) (`self.MaxHealth`))))

(fn `Update Water Level`
  (bind _aswater_level_bar (cast `/Game/UI/UI_Widgets/Water_Level_Bar` (`WidgetComponent.GetWidget` (`self.Water_Level_Bar_Widget`))))
  (`ProgressBar.SetPercent` (`/Game/UI/UI_Widgets/Water_Level_Bar.Water_Level_Pumpkin` _aswater_level_bar) (/ (`self.CurrentWater`) (`self.MaxWater`))))

(fn `UserConstructionScript`)