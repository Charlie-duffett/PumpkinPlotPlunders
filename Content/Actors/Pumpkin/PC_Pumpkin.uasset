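; AI controller for the pumpkin actor that runs the BT_PumpkinAI behavior tree and feeds its blackboard.
; On BeginPlay it sets player character 0 as TargetActor and starts with the evil flag off.
; It listens for that character's destruction to set BIsPlayerDestroyed.
; SetIsEvil lets the evil flag be changed through the blackboard.
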(event `self.ReceiveBeginPlay`
  (bind _blackboard (`self.Blackboard`))
  (add `self.OnDestroyed` (`GameplayStatics.GetPlayerCharacter` 0) (delegate `On Player Destoryed`))
  (`self.RunBehaviorTree` "/Game/Actors/Pumpkin/BT_PumpkinAI.BT_PumpkinAI")
  (`BlackboardComponent.SetValueAsObject` _blackboard (`self.TargetActor`) (`GameplayStatics.GetPlayerCharacter` 0))
  (`BlackboardComponent.SetValueAsBool` _blackboard (`self.bIsEvil`) false))

(event `On Player Destoryed` :!signature `self.OnDestroyed`
  (params (DestroyedActor :type "Actor Object Reference"))
  (`BlackboardComponent.SetValueAsBool` (`self.Blackboard`) (`self.bIsPlayerDestroyed`) true))

(fn `SetIsEvil`
  (params (IsEvil :type Boolean))
  (`BlackboardComponent.SetValueAsBool` (`self.Blackboard`) (`self.bIsEvil`) IsEvil))

(fn `UserConstructionScript`)